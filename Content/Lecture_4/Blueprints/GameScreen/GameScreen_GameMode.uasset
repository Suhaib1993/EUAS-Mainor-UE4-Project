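; Game mode for the game screen that sets up player input for gameplay and provides the death screen.
; On BeginPlay it hides the mouse cursor and switches the first player controller to game-only input.
; Its DeathScreen event creates and stores a UMG_Death widget, adds it to the viewport, shows the cursor and switches to UI-only input without mouse lock.
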(event `self.ReceiveBeginPlay`
  (bind _returnvalue (`GameplayStatics.GetPlayerController` 0))
  (set `PlayerController.bShowMouseCursor` false _returnvalue)
  (`WidgetBlueprintLibrary.SetInputMode_GameOnly` _returnvalue))

(event `DeathScreen`
  (bind _returnvalue (`GameplayStatics.GetPlayerController` 0))
  (bind _returnvalue_2 (`|CreateWidget` "/Game/Lecture_4/Blueprints/GameScreen/UMG_Death.UMG_Death_C"))
  (set `self.Death_Ref` _returnvalue_2)
  (`UserWidget.AddToViewport` (`self.Death_Ref`) 0)
  (set `PlayerController.bShowMouseCursor` true _returnvalue)
  (`WidgetBlueprintLibrary.SetInputMode_UIOnlyEx` _returnvalue null))

(fn `UserConstructionScript`)